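; Spawn handler that caps how many patrons are in the level and scales spawning difficulty.
; The construction script finds the spawner and door; BeginPlay binds spawn events from the spawner and despawn events from the door and cat player controller.
; Each event updates the patron count, toggling the spawner off at capacity and on below it.
; An increase-difficulty event shortens spawn cooldowns and raises the cap.
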(event Custom|increase-difficulty
  (bind _spawner_ref (Variables|Default|Getspawner-ref))
  (bind _spawner_ref_2 (Variables|Default|Getspawner-ref))
  (Variables|/Game/Blueprints/Objects/bp-spawner.bp-spawner_C|Setmax-cooldown _spawner_ref_2 (- (Variables|/Game/Blueprints/Objects/bp-spawner.bp-spawner_C|Getmax-cooldown _spawner_ref_2) 0.5))
  (Variables|/Game/Blueprints/Objects/bp-spawner.bp-spawner_C|Setmin-cooldown _spawner_ref (- (Variables|/Game/Blueprints/Objects/bp-spawner.bp-spawner_C|Getmin-cooldown _spawner_ref) 0.05))
  (Variables|Default|Setmax-patrons (+ (Variables|Default|Getmax-patrons) 3))
  (Development|PrintString "Increased Difficulty"))

(event Custom|spawned-patron
  (bind _result (Math|Integer|IncrementInt (Variables|Default|Getspawned-patrons))
    (:%20%20
      (CallFunction|Check-at-capacity))))

(event Custom|despawned-patron
  (bind _result (Math|Integer|DecrementInt (Variables|Default|Getspawned-patrons))
    (:%20%20
      (Development|PrintString (Utilities|String|ToString(Integer) _result))
      (CallFunction|Check-at-capacity))))

(event Custom|check-at-capacity
  (if (>= (Variables|Default|Getspawned-patrons) (Variables|Default|Getmax-patrons))
    (Variables|/Game/Blueprints/Objects/bp-spawner.bp-spawner_C|Setis-active (Variables|Default|Getspawner-ref) false)
    (else
      (Variables|/Game/Blueprints/Objects/bp-spawner.bp-spawner_C|Setis-active (Variables|Default|Getspawner-ref) true))))

(event EventBeginPlay
  (EventDispatchers|BindEventtoSpawned-patron (Variables|Default|Getspawner-ref) (delegate Custom|spawned-patron))
  (EventDispatchers|BindEventtoPatron-gone (Variables|Default|Getdoor-ref) (delegate Custom|despawned-patron))
  (bind _ascat_playercontroller (Utilities|Casting|CastTocat-playercontroller (Game|GetPlayerController 0)))
  (EventDispatchers|BindEventtoDespawn-patron _ascat_playercontroller (delegate Custom|despawned-patron))
  (Variables|/Game/Blueprints/Objects/bp-spawner.bp-spawner_C|Setis-active (Variables|Default|Getspawner-ref) true))

(fn ConstructionScript
  (bind _outactors (Actor|GetAllActorsOfClass "/Game/Blueprints/Objects/bp-spawner.bp-spawner_C"))
  (Variables|Default|Setspawner-ref (Utilities|Array|Get(acopy) _outactors))
  (bind _outactors_2 (Actor|GetAllActorsOfClass "/Game/Blueprints/Objects/bp-door.bp-door_C"))
  (Variables|Default|Setdoor-ref (Utilities|Array|Get(acopy) _outactors_2)))