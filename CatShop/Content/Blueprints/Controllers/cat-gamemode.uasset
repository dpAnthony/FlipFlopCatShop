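; Game mode for a cat game that runs the match timer, score state and stepped difficulty.
; Start-game creates the score widget and resets state, while start-time lets Tick advance the timer, push it to the UI and call Gameovered when score reaches zero.
; Tick samples a difficulty curve by elapsed time, and exact values 1 to 10 each fire a DoOnce that raises level and Onichance and notifies the spawn handler.
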(event Custom|start-game
  (bind _returnvalue (UserInterface|CreateWidget "/Game/Widgets/ui-score.ui-score_C" (Game|GetPlayerController 0)))
  (UserInterface|Viewport|AddtoViewport _returnvalue 0)
  (Variables|Default|Setui-score-ref _returnvalue)
  (Variables|Default|Setgame-time 0.0)
  (Variables|Default|Setscore-total 1)
  (Variables|Default|Setoni-chance 50)
  (Variables|Default|Setdifficulty-level 0)
  (Variables|Default|Setgame-started true))

(event Custom|start-time
  (Variables|Default|Settime-started true))

(event EventBeginPlay)

(event EventTick
  (params (DeltaSeconds :type Float%20%28single-precision%29))
  (if (Variables|Default|Getgame-started)
    (if (Variables|Default|Gettime-started)
      (Variables|Default|Setgame-time (+ DeltaSeconds (Variables|Default|Getgame-time)))
      (Utilities|FlowControl|Sequence
        (:then_0
          (if (<= (Variables|Default|Getscore-total) 0)
            (Default|CallGame-over-ed)))
        (:then_1
          (Variables|/Game/Widgets/ui-score.ui-score_C|Settime (Variables|Default|Getui-score-ref) (Variables|Default|Getgame-time)))
        (:then_2
          (if (== (Math|Curves|GetFloatValue (Variables|Default|Getdifficulty-curve-fast) (Variables|Default|Getgame-time)) 1.0)
            (Utilities|FlowControl|DoOnce false
              (:Completed
                (Math|Integer|IncrementInt (Variables|Default|Getdifficulty-level)
                  (:%20%20
                    (Variables|Default|Setoni-chance (+ (Variables|Default|Getoni-chance) 5))
                    (Default|Increase-difficulty (Variables|Default|Getspawnhandler-ref))
                    (Development|PrintString "1")))))
            (elif (== (Math|Curves|GetFloatValue (Variables|Default|Getdifficulty-curve-fast) (Variables|Default|Getgame-time)) 2.0)
              (Utilities|FlowControl|DoOnce false
                (:Completed
                  (Math|Integer|IncrementInt (Variables|Default|Getdifficulty-level)
                    (:%20%20
                      (Variables|Default|Setoni-chance (+ (Variables|Default|Getoni-chance) 5))
                      (Default|Increase-difficulty (Variables|Default|Getspawnhandler-ref))
                      (Development|PrintString "2")))))
              (elif (== (Math|Curves|GetFloatValue (Variables|Default|Getdifficulty-curve-fast) (Variables|Default|Getgame-time)) 3.0)
                (Utilities|FlowControl|DoOnce false
                  (:Completed
                    (Math|Integer|IncrementInt (Variables|Default|Getdifficulty-level)
                      (:%20%20
                        (Variables|Default|Setoni-chance (+ (Variables|Default|Getoni-chance) 5))
                        (Default|Increase-difficulty (Variables|Default|Getspawnhandler-ref))
                        (Development|PrintString "3")))))
                (elif (== (Math|Curves|GetFloatValue (Variables|Default|Getdifficulty-curve-fast) (Variables|Default|Getgame-time)) 4.0)
                  (Utilities|FlowControl|DoOnce false
                    (:Completed
                      (Math|Integer|IncrementInt (Variables|Default|Getdifficulty-level)
                        (:%20%20
                          (Variables|Default|Setoni-chance (+ (Variables|Default|Getoni-chance) 5))
                          (Default|Increase-difficulty (Variables|Default|Getspawnhandler-ref))
                          (Development|PrintString "4")))))
                  (elif (== (Math|Curves|GetFloatValue (Variables|Default|Getdifficulty-curve-fast) (Variables|Default|Getgame-time)) 5.0)
                    (Utilities|FlowControl|DoOnce false
                      (:Completed
                        (Math|Integer|IncrementInt (Variables|Default|Getdifficulty-level)
                          (:%20%20
                            (Variables|Default|Setoni-chance (+ (Variables|Default|Getoni-chance) 5))
                            (Default|Increase-difficulty (Variables|Default|Getspawnhandler-ref))
                            (Development|PrintString "5")))))
                    (elif (== (Math|Curves|GetFloatValue (Variables|Default|Getdifficulty-curve-fast) (Variables|Default|Getgame-time)) 6.0)
                      (Utilities|FlowControl|DoOnce false
                        (:Completed
                          (Math|Integer|IncrementInt (Variables|Default|Getdifficulty-level)
                            (:%20%20
                              (Variables|Default|Setoni-chance (+ (Variables|Default|Getoni-chance) 5))
                              (Default|Increase-difficulty (Variables|Default|Getspawnhandler-ref))
                              (Development|PrintString "6")))))
                      (elif (== (Math|Curves|GetFloatValue (Variables|Default|Getdifficulty-curve-fast) (Variables|Default|Getgame-time)) 7.0)
                        (Utilities|FlowControl|DoOnce false
                          (:Completed
                            (Math|Integer|IncrementInt (Variables|Default|Getdifficulty-level)
                              (:%20%20
                                (Variables|Default|Setoni-chance (+ (Variables|Default|Getoni-chance) 5))
                                (Default|Increase-difficulty (Variables|Default|Getspawnhandler-ref))
                                (Development|PrintString "7")))))
                        (elif (== (Math|Curves|GetFloatValue (Variables|Default|Getdifficulty-curve-fast) (Variables|Default|Getgame-time)) 8.0)
                          (Utilities|FlowControl|DoOnce false
                            (:Completed
                              (Math|Integer|IncrementInt (Variables|Default|Getdifficulty-level)
                                (:%20%20
                                  (Variables|Default|Setoni-chance (+ (Variables|Default|Getoni-chance) 5))
                                  (Default|Increase-difficulty (Variables|Default|Getspawnhandler-ref))
                                  (Development|PrintString "8")))))
                          (elif (== (Math|Curves|GetFloatValue (Variables|Default|Getdifficulty-curve-fast) (Variables|Default|Getgame-time)) 9.0)
                            (Utilities|FlowControl|DoOnce false
                              (:Completed
                                (Math|Integer|IncrementInt (Variables|Default|Getdifficulty-level)
                                  (:%20%20
                                    (Variables|Default|Setoni-chance (+ (Variables|Default|Getoni-chance) 5))
                                    (Default|Increase-difficulty (Variables|Default|Getspawnhandler-ref))
                                    (Development|PrintString "9")))))
                            (elif (== (Math|Curves|GetFloatValue (Variables|Default|Getdifficulty-curve-fast) (Variables|Default|Getgame-time)) 1e+01)
                              (Utilities|FlowControl|DoOnce false
                                (:Completed
                                  (Math|Integer|IncrementInt (Variables|Default|Getdifficulty-level)
                                    (:%20%20
                                      (Variables|Default|Setoni-chance (+ (Variables|Default|Getoni-chance) 5))
                                      (Default|Increase-difficulty (Variables|Default|Getspawnhandler-ref))
                                      (Development|PrintString "10"))))))))))))))))))))

(fn ConstructionScript)

(fn Update-score-ui
  (Variables|/Game/Widgets/ui-score.ui-score_C|Setscore (Variables|Default|Getui-score-ref) (Variables|Default|Getscore-total)))