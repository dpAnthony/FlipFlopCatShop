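; Player controller for the cat game, handling flip, flop, spook and quit input.
; Flip and flop call the player's matching action and set which zone is active.
; Releasing spook with anyone in either zone plays the active side's flipbook and sound, then restores idle after a delay.
; It kills yokai and spooks other people in the active zone, calling Despawnpatron for each.
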(event EventBeginPlay
  (bind _ascat_gamemode (Utilities|Casting|CastTocat-gamemode (Game|GetGameMode)))
  (Variables|Default|Setgamemode-ref _ascat_gamemode))

(event Input|ActionEvents|InputActionflip
  (params (Key :type Key%20Structure))
  (:Pressed
    (Default|Flip (Variables|Default|Getplayer-ref))
    (Variables|Default|Setzone-state 1)))

(event Input|ActionEvents|InputActionflop
  (params (Key :type Key%20Structure))
  (:Pressed
    (Default|Flop (Variables|Default|Getplayer-ref))
    (Variables|Default|Setzone-state 0)))

(event Input|ActionEvents|InputActionspook
  (params (Key :type Key%20Structure))
  (bind _player_ref (Variables|Default|Getplayer-ref))
  (bind _player_ref_2 (Variables|Default|Getplayer-ref))
  (bind _player_ref_3 (Variables|Default|Getplayer-ref))
  (bind _player_ref_4 (Variables|Default|Getplayer-ref))
  (bind _flip_sprite (Variables|/Game/Blueprints/Objects/obj-player.obj-player_C|Getflip-sprite _player_ref_4))
  (bind _flop_sprite (Variables|/Game/Blueprints/Objects/obj-player.obj-player_C|Getflop-sprite _player_ref))
  (bind _flop_sprite_2 (Variables|/Game/Blueprints/Objects/obj-player.obj-player_C|Getflop-sprite _player_ref_3))
  (bind _flip_sprite_2 (Variables|/Game/Blueprints/Objects/obj-player.obj-player_C|Getflip-sprite _player_ref_2))
  (:Released
    (if (or (> (Utilities|Array|Length (Collision|GetOverlappingActors (Variables|/Game/Blueprints/Objects/bp-flop-zone.bp-flop-zone_C|Getflop-spook-zone (Variables|Default|Getzone-0)) "/Game/Blueprints/Objects/obj-person.obj-person_C" :!class /Script/Engine.PrimitiveComponent)) 0) (> (Utilities|Array|Length (Collision|GetOverlappingActors (Variables|/Game/Blueprints/Objects/bp-flip-zone.bp-flip-zone_C|Getflip-spook-zone (Variables|Default|Getzone-1)) "/Game/Blueprints/Objects/obj-person.obj-person_C" :!class /Script/Engine.PrimitiveComponent)) 0))
      (switch int (Variables|Default|Getzone-state)
        (:0
          (Sprite|SetFlipbook _flop_sprite "/Game/Materials/Sprites/flop-cat/fb-flop-spook.fb-flop-spook")
          (Components|Timeline|PlayfromStart _flop_sprite)
          (Audio|PlaySound2D "/Game/retro_8bit_sounds/damage_hurt/Cues/flip-spook-sound.flip-spook-sound" 1.0 1.0 0.0 0 0)
          (for _array_element (Collision|GetOverlappingActors (Variables|/Game/Blueprints/Objects/bp-flop-zone.bp-flop-zone_C|Getflop-spook-zone (Variables|Default|Getzone-0)) "/Game/Blueprints/Objects/obj-person.obj-person_C" :!class /Script/Engine.PrimitiveComponent)
            (bind _asobj_person (Utilities|Casting|CastToobj-person _array_element))
            (if (Variables|/Game/Blueprints/Objects/obj-person.obj-person_C|Getis-yokai _asobj_person)
              (Default|Yokai-death _asobj_person)
              (else
                (Default|Spook-person _asobj_person)))
            (Default|CallDespawn-patron))
          (Utilities|FlowControl|Delay (Class|PaperFlipbookComponent|GetFlipbookLength _flop_sprite_2))
          (Sprite|SetFlipbook _flop_sprite_2 "/Game/Materials/Sprites/flop-cat/fb-flop-idle.fb-flop-idle"))
        (:1
          (Sprite|SetFlipbook _flip_sprite "/Game/Materials/Sprites/flip-cat/fb-flip-spook.fb-flip-spook")
          (Components|Timeline|PlayfromStart _flip_sprite)
          (Audio|PlaySound2D "/Game/retro_8bit_sounds/damage_hurt/Cues/flop-spook-sound.flop-spook-sound" 1.0 1.0 0.0 0 0)
          (for _array_element_2 (Collision|GetOverlappingActors (Variables|/Game/Blueprints/Objects/bp-flip-zone.bp-flip-zone_C|Getflip-spook-zone (Variables|Default|Getzone-1)) "/Game/Blueprints/Objects/obj-person.obj-person_C" :!class /Script/Engine.PrimitiveComponent)
            (bind _asobj_person_2 (Utilities|Casting|CastToobj-person _array_element_2))
            (if (Variables|/Game/Blueprints/Objects/obj-person.obj-person_C|Getis-yokai _asobj_person_2)
              (Default|Yokai-death _asobj_person_2)
              (else
                (Default|Spook-person _asobj_person_2)))
            (Default|CallDespawn-patron))
          (Utilities|FlowControl|Delay (Class|PaperFlipbookComponent|GetFlipbookLength _flip_sprite_2))
          (Sprite|SetFlipbook _flip_sprite_2 "/Game/Materials/Sprites/flip-cat/fb-flip-idle.fb-flip-idle"))))))

(event Input|ActionEvents|InputActionexit
  (params (Key :type Key%20Structure))
  (:Pressed
    (Game|QuitGame 0 "Quit" false)))

(fn ConstructionScript)