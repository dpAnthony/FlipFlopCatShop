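; Door actor that scores each person entering its Box trigger and then removes them from the level.
; On BeginPlay it caches the cat game mode.
; When an obj-person overlaps the Box, its Isoni flag decides whether the game mode's total score takes a penalty or a smaller reward.
; It then destroys that person and has the game mode refresh the score UI.
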(event OnComponentBeginOverlap(Box)
  (params (OverlappedComponent :type Primitive%20Component%20Object%20Reference) (OtherActor :type Actor%20Object%20Reference) (OtherComp :type Primitive%20Component%20Object%20Reference) (OtherBodyIndex :type Integer) (bFromSweep :type Boolean) (SweepResult :type Hit%20Result%20Structure%20%28by%20ref%29))
  (bind _gamemode_ref (Variables|Default|Getgamemode-ref))
  (bind _gamemode_ref_2 (Variables|Default|Getgamemode-ref))
  (bind _asobj_person (Utilities|Casting|CastToobj-person OtherActor))
  (if (Variables|/Game/Blueprints/Objects/obj-person.obj-person_C|Getis-oni _asobj_person)
    (Variables|/Game/Blueprints/Controllers/cat-gamemode.cat-gamemode_C|Setscore-total _gamemode_ref (- (Variables|/Game/Blueprints/Controllers/cat-gamemode.cat-gamemode_C|Getscore-total _gamemode_ref) 10))
    (else
      (Variables|/Game/Blueprints/Controllers/cat-gamemode.cat-gamemode_C|Setscore-total _gamemode_ref_2 (+ (Variables|/Game/Blueprints/Controllers/cat-gamemode.cat-gamemode_C|Getscore-total _gamemode_ref_2) 5))))
  (Actor|DestroyActor _asobj_person)
  (Default|Update-score-ui (Variables|Default|Getgamemode-ref)))

(event EventBeginPlay
  (bind _ascat_gamemode (Utilities|Casting|CastTocat-gamemode (Game|GetGameMode)))
  (Variables|Default|Setgamemode-ref _ascat_gamemode))

(event Collision|EventActorBeginOverlap
  (params (OtherActor :type Actor%20Object%20Reference)))

(event EventTick
  (params (DeltaSeconds :type Float%20%28single-precision%29)))

(fn ConstructionScript)