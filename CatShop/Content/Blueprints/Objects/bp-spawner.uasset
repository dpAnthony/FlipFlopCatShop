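; Patron spawner that creates person actors at two points, SpawnL and SpawnR, each with its own cooldown.
; BeginPlay puts one random side on a delayed cooldown to stagger the start.
; While active, Tick attempts a spawn, favoring left over right, calls Spawnedpatron, then starts that side's cooldown.
; Delays come from Randomdelayinrange, whose graph shows only unused random min/max cooldown expressions.
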(event Custom|spawn-patron
  (if (Variables|Default|Geton-cooldown-l)
    (if (not (Variables|Default|Geton-cooldown-r))
      (Game|SpawnActorfromClass "/Game/Blueprints/Objects/obj-person.obj-person_C" (Transformation|GetWorldTransform (Variables|Default|Getspawn-R)) "Undefined" 0 0)
      (Default|CallSpawned-patron)
      (Variables|Default|Seton-cooldown-r true)
      (Utilities|FlowControl|Delay (Utilities|Random-delay-in-range))
      (Variables|Default|Seton-cooldown-r false))
    (else
      (Game|SpawnActorfromClass "/Game/Blueprints/Objects/obj-person.obj-person_C" (Transformation|GetWorldTransform (Variables|Default|Getspawn-L)) "Undefined" 0 0)
      (Default|CallSpawned-patron)
      (Variables|Default|Seton-cooldown-l true)
      (Utilities|FlowControl|Delay (Utilities|Random-delay-in-range))
      (Variables|Default|Seton-cooldown-l false))))

(event EventBeginPlay
  (if (>= (Math|Random|RandomIntegerinRange 0 100) 50)
    (Variables|Default|Seton-cooldown-l true)
    (Utilities|FlowControl|Delay (Utilities|Random-delay-in-range))
    (Variables|Default|Seton-cooldown-l false)
    (else
      (Variables|Default|Seton-cooldown-r true)
      (Utilities|FlowControl|Delay (Utilities|Random-delay-in-range))
      (Variables|Default|Seton-cooldown-r false))))

(event EventTick
  (params (DeltaSeconds :type Float%20%28single-precision%29))
  (if (Variables|Default|Getis-active)
    (CallFunction|Spawn-patron)))

(fn ConstructionScript)