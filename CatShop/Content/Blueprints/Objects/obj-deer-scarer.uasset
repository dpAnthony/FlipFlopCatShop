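; Animated deer scarer prop built on a Paper2D flipbook, with water and tonk sounds.
; On BeginPlay it turns off flipbook looping, adds two audio components and starts the water cue.
; Each time the flipbook finishes, it plays the tonk cue, waits a fixed delay and replays from the start, forming a repeating cycle with a pause.
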(event OnFinishedPlaying(PaperFlipbook)
  (Audio|Components|Audio|Play (Variables|Default|Gettonk-cue) 0.0)
  (Utilities|FlowControl|Delay 4.0)
  (Components|Timeline|PlayfromStart (Variables|Default|GetPaperFlipbook)))

(event EventBeginPlay
  (Components|Timeline|SetLooping (Variables|Default|GetPaperFlipbook) false)
  (bind _returnvalue (AddComponent|AddAudioComponent false))
  (bind _output_get (Variables|Default|Setwater-cue _returnvalue))
  (Audio|Components|Audio|Play _output_get 0.0)
  (bind _returnvalue_2 (AddComponent|AddAudioComponent false))
  (Variables|Default|Settonk-cue _returnvalue_2))

(fn ConstructionScript)