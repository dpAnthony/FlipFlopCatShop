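; Walking person actor, randomly a human or a yokai (oni) by the game mode's Onichance, that moves along X toward center until it reaches the door.
; BeginPlay flips the layered sprites for positive-X spawns, then picks adult, child or one of three yokai builders.
; Builders randomize body, head, hair, clothes and accessories from sprite-array index ranges.
; A cleanup event hides clashing layers in adult and yokai looks.
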(event Custom|make-adult
  (if (< (Math|Random|RandomIntegerinRange 1 100) 70)
    (Utilities|Make-person-adult)
    (else
      (Utilities|Make-person-child))))

(event Custom|make-yokai
  (if (< (Math|Random|RandomIntegerinRange 1 100) 70)
    _
    (else
      _))
  (switch int (Math|Random|RandomIntegerinRange 0 3)
    (:0
      (Utilities|Make-yokai-adult-var-1))
    (:1
      (Utilities|Make-yokai-adult-var-2))
    (:2
      (Utilities|Make-yokai-adult-var-3))))

(event Custom|cleanup-sprite
  (bind _person_head (Variables|Default|Getperson-head))
  (bind _person_acc_m_1 (Variables|Default|Getperson-acc-m-1))
  (bind _person_head_2 (Variables|Default|Getperson-head))
  (bind _returnvalue (Sprite|GetSprite _person_head))
  (bind _returnvalue_2 (Sprite|GetSprite _person_acc_m_1))
  (bind _returnvalue_3 (Sprite|GetSprite _person_head_2))
  (if (Math|Boolean|ORBoolean (== _returnvalue_2 "/Game/Materials/Sprites/person-acc/acc-m-p-1.acc-m-p-1") (== _returnvalue_2 "/Game/Materials/Sprites/person-acc/acc-m-p-2.acc-m-p-2") (== _returnvalue_2 "/Game/Materials/Sprites/person-acc/acc-m-p-3.acc-m-p-3") (== _returnvalue_2 "/Game/Materials/Sprites/yokai-acc/acc-m-y-1.acc-m-y-1") (== _returnvalue_3 "/Game/Materials/Sprites/yokai-base/head-y-3.head-y-3") (== _returnvalue_3 "/Game/Materials/Sprites/yokai-base/head-y-4.head-y-4"))
    (Rendering|SetVisibility (Variables|Default|Getperson-hair) false false))
  (if (and (== (Sprite|GetSprite (Variables|Default|Getperson-acc-m-2)) "/Game/Materials/Sprites/person-acc/acc-m-p-3.acc-m-p-3") (or (== _returnvalue "/Game/Materials/Sprites/yokai-base/head-y-3.head-y-3") (== _returnvalue "/Game/Materials/Sprites/yokai-base/head-y-4.head-y-4")))
    (Rendering|SetVisibility (Variables|Default|Getperson-acc-m-2) false false)))

(event Custom|flip-sprites
  (bind _person_acc_m_2 (Variables|Default|Getperson-acc-m-2))
  (bind _person_acc_f (Variables|Default|Getperson-acc-f))
  (bind _person_acc_m_1 (Variables|Default|Getperson-acc-m-1))
  (bind _person_acc_b (Variables|Default|Getperson-acc-b))
  (bind _person_body (Variables|Default|Getperson-body))
  (bind _person_clothes (Variables|Default|Getperson-clothes))
  (bind _person_head (Variables|Default|Getperson-head))
  (bind _person_hair (Variables|Default|Getperson-hair))
  (bind _relativelocation (Variables|/Script/Engine.SceneComponent|GetRelativeLocation _person_acc_m_2))
  (bind _relativelocation_2 (Variables|/Script/Engine.SceneComponent|GetRelativeLocation _person_acc_f))
  (bind _relativelocation_3 (Variables|/Script/Engine.SceneComponent|GetRelativeLocation _person_acc_m_1))
  (bind _relativelocation_4 (Variables|/Script/Engine.SceneComponent|GetRelativeLocation _person_acc_b))
  (bind _relativelocation_5 (Variables|/Script/Engine.SceneComponent|GetRelativeLocation _person_body))
  (bind _relativelocation_6 (Variables|/Script/Engine.SceneComponent|GetRelativeLocation _person_clothes))
  (bind _relativelocation_7 (Variables|/Script/Engine.SceneComponent|GetRelativeLocation _person_head))
  (bind _relativelocation_8 (Variables|/Script/Engine.SceneComponent|GetRelativeLocation _person_hair))
  (Transformation|SetRelativeRotation (Variables|Default|Getperson-base) "0,180.000000, 0" false false)
  (Transformation|SetRelativeLocation _person_body (Math|Vector|MakeVector (.x _relativelocation_5) (* (.y _relativelocation_5) -1.0) (.z _relativelocation_5)) false false)
  (Transformation|SetRelativeLocation _person_clothes (Math|Vector|MakeVector (.x _relativelocation_6) (* (.y _relativelocation_6) -1.0) (.z _relativelocation_6)) false false)
  (Transformation|SetRelativeLocation _person_head (Math|Vector|MakeVector (.x _relativelocation_7) (* (.y _relativelocation_7) -1.0) (.z _relativelocation_7)) false false)
  (Transformation|SetRelativeLocation _person_hair (Math|Vector|MakeVector (.x _relativelocation_8) (* (.y _relativelocation_8) -1.0) (.z _relativelocation_8)) false false)
  (Transformation|SetRelativeLocation _person_acc_f (Math|Vector|MakeVector (.x _relativelocation_2) (* (.y _relativelocation_2) -1.0) (.z _relativelocation_2)) false false)
  (Transformation|SetRelativeLocation _person_acc_m_1 (Math|Vector|MakeVector (.x _relativelocation_3) (* (.y _relativelocation_3) -1.0) (.z _relativelocation_3)) false false)
  (Transformation|SetRelativeLocation _person_acc_b (Math|Vector|MakeVector (.x _relativelocation_4) (* (.y _relativelocation_4) -1.0) (.z _relativelocation_4)) false false)
  (Transformation|SetRelativeLocation _person_acc_m_2 (Math|Vector|MakeVector (.x _relativelocation) (* (.y _relativelocation) -1.0) (.z _relativelocation)) false false))

(event EventBeginPlay
  (Variables|Default|Setmove-speed (Math|Conversions|ToFloat(Integer) (Math|Float|Round (Math|Random|RandomFloatinRange 1.0 1.0))))
  (if (> (.x (Transformation|GetActorLocation)) 0.0)
    (CallFunction|Flip-sprites))
  (bind _ascat_gamemode (Utilities|Casting|CastTocat-gamemode (Game|GetGameMode)))
  (if (<= (Math|Random|RandomIntegerinRange 0 100) (Variables|/Game/Blueprints/Controllers/cat-gamemode.cat-gamemode_C|Getoni-chance _ascat_gamemode))
    (Variables|Default|Setis-oni true)
    (CallFunction|Make-yokai)
    (else
      (Variables|Default|Setis-oni false)
      (CallFunction|Make-adult))))

(event EventTick
  (params (DeltaSeconds :type Float%20%28single-precision%29))
  (if (Math|Vector|NotEqual(Vector) (Transformation|GetActorLocation) (Transformation|GetActorLocation (Variables|Default|Getdoor_ref)) 0.0001)
    (if (< (.x (Transformation|GetActorLocation)) 0.0)
      (Transformation|AddActorLocalOffset (Math|Vector|MakeVector (Variables|Default|Getmove-speed) 0.0 0.0) false false)
      (else
        (Transformation|AddActorLocalOffset (Math|Vector|MakeVector (* (Variables|Default|Getmove-speed) -1.0) 0.0 0.0) false false)))))

(fn ConstructionScript
  (bind _outactors (Actor|GetAllActorsOfClass "/Game/Blueprints/Objects/bp-door.bp-door_C"))
  (Variables|Default|Setdoor_ref (Utilities|Array|Get(acopy) _outactors)))

(fn Set-random-sprite-in-range
  (params (sprite-component :type Paper%20Sprite%20Component%20Object%20Reference) (sprite-array :type Array%20of%20Paper%20Sprite%20Object%20References) (min-range :type Integer) (max-range :type Integer))
  (bind _returnvalue (Math|Random|RandomIntegerinRange min-range max-range))
  (Rendering|Components|Sprite|SetSprite sprite-component (Utilities|Array|Get(acopy) sprite-array _returnvalue))
  (return _returnvalue))