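; Player Blueprint with a two-state flip/flop look, tracked by a State variable.
; Flip and Flop each set the state, show their coin sprite, move their animated sprite to a Y offset and play it from the start, while resetting and stopping the opposite one.
; A separate flipflop graph toggles State and swaps between the two flat player materials.
; Construction stops the flip animation.
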(fn ConstructionScript
  (Audio|Components|Audio|Stop (Variables|Default|Getflip-sprite)))

(fn Flip
  (bind _flop_sprite (Variables|Default|Getflop-sprite))
  (bind _flip_sprite (Variables|Default|Getflip-sprite))
  (bind _relativelocation (Variables|/Script/Engine.SceneComponent|GetRelativeLocation _flop_sprite))
  (bind _relativelocation_2 (Variables|/Script/Engine.SceneComponent|GetRelativeLocation _flip_sprite))
  (Variables|Default|Setstate 1)
  (Rendering|SetVisibility (Variables|Default|Getflip-coin-sprite) true false)
  (Rendering|SetVisibility (Variables|Default|Getflop-coin-sprite) false false)
  (Transformation|SetRelativeLocation _flip_sprite (Math|Vector|MakeVector (.x _relativelocation_2) 2e+01 (.z _relativelocation_2)) false false)
  (Components|Timeline|PlayfromStart _flip_sprite)
  (Transformation|SetRelativeLocation _flop_sprite (Math|Vector|MakeVector (.x _relativelocation) 0.0 (.z _relativelocation)) false false)
  (Audio|Components|Audio|Stop _flop_sprite))

(fn Flop
  (bind _flip_sprite (Variables|Default|Getflip-sprite))
  (bind _flop_sprite (Variables|Default|Getflop-sprite))
  (bind _relativelocation (Variables|/Script/Engine.SceneComponent|GetRelativeLocation _flip_sprite))
  (bind _relativelocation_2 (Variables|/Script/Engine.SceneComponent|GetRelativeLocation _flop_sprite))
  (Variables|Default|Setstate 0)
  (Rendering|SetVisibility (Variables|Default|Getflop-coin-sprite) true false)
  (Rendering|SetVisibility (Variables|Default|Getflip-coin-sprite) false false)
  (Transformation|SetRelativeLocation _flop_sprite (Math|Vector|MakeVector (.x _relativelocation_2) 2e+01 (.z _relativelocation_2)) false false)
  (Components|Timeline|PlayfromStart _flop_sprite)
  (Transformation|SetRelativeLocation _flip_sprite (Math|Vector|MakeVector (.x _relativelocation) 0.0 (.z _relativelocation)) false false)
  (Audio|Components|Audio|Stop _flip_sprite))