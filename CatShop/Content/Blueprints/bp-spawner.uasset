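; Spawner actor that repeatedly spawns an instance of the Objperson class at its own transform.
; Tick calls the spawn-person graph every frame, and an Oncooldown flag lets it act only when no cooldown is running.
; After each spawn, a Delay of random length between one second and Cooldowntime runs before the flag clears.
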(event EventTick
  (params (DeltaSeconds :type Float%20%28single-precision%29))
  (Utilities|Spawn-person))

(fn ConstructionScript)